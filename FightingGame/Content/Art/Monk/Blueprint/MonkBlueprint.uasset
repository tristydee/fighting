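; MonkBlueprint is a 2D Monk character driven by PaperZD animation, with movement and attack input.
; BeginPlay registers the FightingInput Enhanced Input mapping context with its player controller.
; Move input drives movement along world X and prints its value.
; Attack jumps the animation instance to its Attack node, using a DoOnce that resets just before the sprite's flipbook length elapses to block repeated triggers.
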(event `self.ReceiveBeginPlay`
  (bind _asplayer_controller (cast `PlayerController` (`self.GetController`)))
  (bind _returnvalue (pcsubsystem `EnhancedInputLocalPlayerSubsystem` _asplayer_controller))
  (`/Engine/EditorBlueprintResources/StandardMacros.IsValid` _returnvalue
    (:`Is Valid`
      (`EnhancedInputSubsystemInterface.AddMappingContext` _returnvalue "/Game/Controls/FightingInput.FightingInput" 0 (struct)))))

(event `EnhancedInput|/Game/Controls/Move_IA`
  (params (ActionValue :type "Float (double-precision)") (ElapsedSeconds :type "Float (double-precision)") (TriggeredSeconds :type "Float (double-precision)") (InputAction :type "InputAction Object Reference" :default "/Game/Controls/Move_IA.Move_IA"))
  (:`Triggered`
    (`KismetSystemLibrary.PrintString` (`KismetStringLibrary.Conv_DoubleToString` ActionValue))
    (`self.AddMovementInput` (1.0 0.0 0.0) ActionValue)))

(event `EnhancedInput|/Game/Controls/Attack_IA`
  (params (ActionValue :type Boolean) (ElapsedSeconds :type "Float (double-precision)") (TriggeredSeconds :type "Float (double-precision)") (InputAction :type "InputAction Object Reference" :default "/Game/Controls/Attack_IA.Attack_IA"))
  (:`Started`
    (`/Engine/EditorBlueprintResources/StandardMacros.DoOnce` false :!label _label
      (:`Completed`
        (`PaperZDAnimInstance.JumpToNode` (`PaperZDAnimationComponent.AnimInstance` (`self.AnimationComponent`)) "Attack" "None")
        (`KismetSystemLibrary.Delay` (- (`PaperFlipbookComponent.GetFlipbookLength` (`self.Sprite`)) 0.1))
        (goto _label :!via `Reset`)))))

(fn `UserConstructionScript`)